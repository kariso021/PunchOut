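; BP_OfficeCharacter is the player character for an office, able to crouch and to sit on or leave seats.
; E calls a server event that picks the nearest usable tagged BP_OfficeSeat within range, occupies it and teleports the character there, saving a standing transform for getting up.
; An IsSeated RepNotify toggles collision and movement mode, while Left Ctrl toggles crouch unless seated.
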(event `ServerToggleSeat`
  (`self.ToggleSeatAuthority`))

(event `Key|LeftControl`
  (params (Key :type "Key Structure"))
  (:`Pressed`
    (`self.ToggleCrouch`)))

(event `Key|E`
  (params (Key :type "Key Structure"))
  (:`Pressed`
    (`self.ServerToggleSeat`)))

(fn `ApplySeatedState`
  (bind _charactermovement (`self.CharacterMovement`))
  (if (`self.IsSeated`)
    (`self.UnCrouch`)
    (`MovementComponent.StopMovementImmediately` _charactermovement)
    (`self.SetActorEnableCollision` false)
    (`CharacterMovementComponent.SetMovementMode` _charactermovement "MOVE_None" 0)
    (else
      (`self.SetActorEnableCollision` true)
      (`CharacterMovementComponent.SetMovementMode` _charactermovement "MOVE_Walking" 0))))

(fn `OnRep_IsSeated`
  (`self.ApplySeatedState`))

(fn `ToggleCrouch`
  (if (not (`self.IsSeated`))
    (if (`self.bIsCrouched`)
      (`self.UnCrouch`)
      (else
        (`self.Crouch`)))))

(fn `ToggleSeatAuthority`
  (bind _nearestseat (`self.NearestSeat`))
  (if (`self.IsSeated`)
    (`/Game/Office/Blueprints/BP_OfficeSeat.ReleaseSeat` (`self.CurrentSeat`))
    (`self.K2_SetActorTransform` (`self.StandingTransform`) false true)
    (set `self.IsSeated` false)
    (else
      (set `self.NearestSeat` null)
      (set `self.NearestSeatDistance` 170.0)
      (bind _outactors (`GameplayStatics.GetAllActorsWithTag` "OfficeSeat"))
      (for _array_element _outactors
        (bind _asbp_office_seat (cast `/Game/Office/Blueprints/BP_OfficeSeat` _array_element))
        (bind _available (`/Game/Office/Blueprints/BP_OfficeSeat.CanUseSeat` _asbp_office_seat))
        (bind _returnvalue (`self.GetDistanceTo` _asbp_office_seat))
        (if (and _available (< _returnvalue (`self.NearestSeatDistance`)))
          (set `self.NearestSeat` _asbp_office_seat)
          (set `self.NearestSeatDistance` _returnvalue)))
      (`/Engine/EditorBlueprintResources/StandardMacros.IsValid` _nearestseat
        (:`Is Valid`
          (set `self.StandingTransform` (`KismetMathLibrary.MakeTransform` (+ (`self.K2_GetActorLocation`) (`KismetMathLibrary.MakeVector` 0.0 0.0 (select `bool` (`self.bIsCrouched`) :`false` 0.0 :`true` 30.0))) (`self.K2_GetActorRotation`)))
          (set `self.CurrentSeat` _nearestseat)
          (`/Game/Office/Blueprints/BP_OfficeSeat.OccupySeat` _nearestseat)
          (set `self.IsSeated` true)
          (`self.K2_SetActorLocationAndRotation` (`self.K2_GetActorLocation` _nearestseat) (`self.K2_GetActorRotation` _nearestseat) false true))))))

(fn `UserConstructionScript`
  (`parent.UserConstructionScript`))